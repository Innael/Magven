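; Magventures game mode that creates the BP_BattleSystem at BeginPlay and handles its player action callbacks.
; Main and second-weapon attacks flag the character's action, play a swing sound for swords, blink the battle UI, then after a delay call back into the battle system.
; Potion use restores health, stamina or mana, refreshes the inventory slot and, after the same blink delay, recalculates inventory and advances the turn.
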(event `PlayerSecondWeaponAttackIndication`
  (params (ActionCode :type Integer) (TargetEnemy :type "Actor Object Reference"))
  (bind _returnvalue (- ActionCode 1))
  (bind _asbp_game_instance (cast `/Game/Magventures/GameInstance/BP_GameInstance` (`GameplayStatics.GetGameInstance`)))
  (bind _output (`|GetArrayItem` (`/Game/Magventures/GameInstance/BP_GameInstance.Char_Arr` _asbp_game_instance) _returnvalue))
  (set `P_Character.PlayerActionTypeInd` 1 _output)
  (bind _ashud_bi (cast `/Game/Magventures/HUD/HUD_BI` (`PlayerController.GetHUD` (`GameplayStatics.GetPlayerController` 0))))
  (bind _aswbp_battle_interface (cast `/Game/Magventures/Widgets/WBP_BattleInterface` (`Magventure_HUD.BattleInterfaceWidgetInstance` _ashud_bi)))
  (`/Game/Magventures/Widgets/WBP_BattleInterface.ItemUsed` _aswbp_battle_interface)
  (bind _secondmeleeweapon (`P_Character.SecondMeleeWeapon` _output))
  (`/Engine/EditorBlueprintResources/StandardMacros.IsValid` _secondmeleeweapon
    (:`Is Valid`
      (switch `EWeaponType` (`WeaponData.WeaponType` _secondmeleeweapon)
        (:`NotWeapon`
          _)
        (:`Hand`
          _)
        (:`Sword`
          (`GameplayStatics.PlaySound2D` "/Game/Magventures/Sound/Effect/Sword_Swing.Sword_Swing" 1.0 1.0 0.0 null null))
        (:`Axe`
          _)
        (:`Mace`
          _)
        (:`Spear`
          _)
        (:`Dagger`
          _)
        (:`Staff`
          _)))
    (:`Is Not Valid`
      _))
  (`/Game/Magventures/Widgets/WBP_BattleInterface.StartBlink` _aswbp_battle_interface _returnvalue)
  (`KismetSystemLibrary.Delay` 5.0)
  (bind _asch_enemy (cast `/Game/Magventures/Enemy/CH_Enemy` TargetEnemy))
  (set `P_Character.PlayerActionTypeInd` 0 _output)
  (`/Game/Magventures/Widgets/WBP_BattleInterface.ItemUsed` _aswbp_battle_interface)
  (`BattleSystem.PlayerSecondWeaponAttack` (`self.BatSys`) _asch_enemy _output))

(event `PlayerAttackIndication`
  (params (ActionCode :type Integer) (TargetEnemy :type "Actor Object Reference"))
  (bind _returnvalue (- ActionCode 1))
  (bind _asbp_game_instance (cast `/Game/Magventures/GameInstance/BP_GameInstance` (`GameplayStatics.GetGameInstance`)))
  (bind _output (`|GetArrayItem` (`/Game/Magventures/GameInstance/BP_GameInstance.Char_Arr` _asbp_game_instance) _returnvalue))
  (set `P_Character.PlayerActionTypeInd` 1 _output)
  (bind _ashud_bi (cast `/Game/Magventures/HUD/HUD_BI` (`PlayerController.GetHUD` (`GameplayStatics.GetPlayerController` 0))))
  (bind _aswbp_battle_interface (cast `/Game/Magventures/Widgets/WBP_BattleInterface` (`Magventure_HUD.BattleInterfaceWidgetInstance` _ashud_bi)))
  (`/Game/Magventures/Widgets/WBP_BattleInterface.ItemUsed` _aswbp_battle_interface)
  (bind _meleeweapon (`P_Character.MeleeWeapon` _output))
  (`/Engine/EditorBlueprintResources/StandardMacros.IsValid` _meleeweapon
    (:`Is Valid`
      (switch `EWeaponType` (`WeaponData.WeaponType` _meleeweapon)
        (:`NotWeapon`
          _)
        (:`Hand`
          _)
        (:`Sword`
          (`GameplayStatics.PlaySound2D` "/Game/Magventures/Sound/Effect/Sword_Swing.Sword_Swing" 1.0 1.0 0.0 null null))
        (:`Axe`
          _)
        (:`Mace`
          _)
        (:`Spear`
          _)
        (:`Dagger`
          _)
        (:`Staff`
          _)))
    (:`Is Not Valid`
      _))
  (`/Game/Magventures/Widgets/WBP_BattleInterface.StartBlink` _aswbp_battle_interface _returnvalue)
  (`KismetSystemLibrary.Delay` 5.0)
  (bind _asch_enemy (cast `/Game/Magventures/Enemy/CH_Enemy` TargetEnemy))
  (set `P_Character.PlayerActionTypeInd` 0 _output)
  (`/Game/Magventures/Widgets/WBP_BattleInterface.ItemUsed` _aswbp_battle_interface)
  (`BattleSystem.PlayerAttack` (`self.BatSys`) _asch_enemy _output))

(event `self.ReceiveBeginPlay`
  (`KismetSystemLibrary.Delay` 0.1)
  (bind _returnvalue (`|GenericCreateObject` "/Game/Magventures/GameLogic/BP_BattleSystem.BP_BattleSystem_C"))
  (bind _output_get (set `self.BatSys` _returnvalue))
  (add `BattleSystem.OnActionRequested` _output_get (delegate `PotionDrink`))
  (add `BattleSystem.OnPlayerAttack` _output_get (delegate `PlayerAttackIndication`))
  (add `BattleSystem.OnPlayerSecondWeaponAttack` _output_get (delegate `PlayerSecondWeaponAttackIndication`)))

(event `PotionDrink`
  (params (SlotIndex :type Integer) (CharIndex :type Integer))
  (bind _returnvalue (- CharIndex 1))
  (bind _asbp_game_instance (cast `/Game/Magventures/GameInstance/BP_GameInstance` (`GameplayStatics.GetGameInstance`)))
  (bind _output_inventoryslots (break `CharacterInventoryPacket` (`|GetArrayItem` (`Magv_GameInstance.PartyInventories` _asbp_game_instance) (- CharIndex 1))))
  (bind (_output_itemdata _output_stackcount) (break `InventorySlotStruct` (`|GetArrayItem` _output_inventoryslots SlotIndex)))
  (`/Engine/EditorBlueprintResources/StandardMacros.IsValid` _output_itemdata
    (:`Is Valid`
      (switch `EItemCategory` (`ItemData.Category` _output_itemdata)
        (:`Potion`
          (bind _aspotion_data (cast `PotionData` _output_itemdata))
          (`GameplayStatics.PlaySound2D` "/Game/Magventures/Sound/Effect/bubble-burst.bubble-burst" 1.0 1.0 0.0 null null)
          (switch `EPotionType` (`PotionData.PotionType` _aspotion_data)
            (:`HealingPotion`
              (bind _char_arr (`/Game/Magventures/GameInstance/BP_GameInstance.Char_Arr` _asbp_game_instance))
              (bind _output (`|GetArrayItem` _char_arr _returnvalue))
              (`P_Character.ChangeHealth` _output (`PotionData.HealthRestore` _aspotion_data)))
            (:`StaminaPotion`
              (`P_Character.ChangeStamina` _output (`PotionData.StaminaRestore` _aspotion_data)))
            (:`ManaPotion`
              (`P_Character.ChangeMana` _output (`PotionData.ManaRestore` _aspotion_data))))
          (bind _ashud_bi (cast `/Game/Magventures/HUD/HUD_BI` (`PlayerController.GetHUD` (`GameplayStatics.GetPlayerController` 0))))
          (bind _returnvalue_2 (- _output_stackcount 1))
          (if (> _returnvalue_2 0)
            (bind _output_2 (`|GetArrayItem` (`/Game/Magventures/Widgets/WBP_CharacterPersonalInventory.SlotWidgetArray` (`/Game/Magventures/Widgets/WBP_CharacterMainWindow.WBP_CharacterPersonalInventory` (`|GetArrayItem` (`/Game/Magventures/HUD/HUD_BI.CharacterWidgets` _ashud_bi) (- CharIndex 1)))) SlotIndex))
            (`/Game/Magventures/Widgets/WBP_InventorySlot.RefreshSlot` _output_2 _returnvalue_2 _output_itemdata)
            (else
              (`/Game/Magventures/Widgets/WBP_InventorySlot.RefreshSlot` _output_2 0 null)
              (`/Game/Magventures/Widgets/WBP_InventorySlot.ClearSlot` _output_2)))
          (bind _aswbp_battle_interface (cast `/Game/Magventures/Widgets/WBP_BattleInterface` (`Magventure_HUD.BattleInterfaceWidgetInstance` _ashud_bi)))
          (`/Game/Magventures/Widgets/WBP_BattleInterface.StartBlink` _aswbp_battle_interface _returnvalue)
          (`KismetSystemLibrary.Delay` 5.0)
          (`Magv_GameInstance.RecalculateInventory` _asbp_game_instance _char_arr)
          (`/Game/Magventures/Widgets/WBP_BattleInterface.ItemUsed` _aswbp_battle_interface)
          (`BattleSystem.NextFighterTurn` (`self.BatSys`)))))))

(fn `UserConstructionScript`)