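; BP_AxeMisslie is a thrown axe projectile whose behavior depends on a ShotResult0 value.
; On BeginPlay it plays a throw sound and launches along local forward, first randomly skewing pitch and yaw for result 2 so the shot veers off.
; On overlapping any actor other than its instigator, it plays a different sound for results 0 and 1, then destroys itself.
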(event `self.ReceiveBeginPlay`
  (switch `int` (`self.ShotResult_0`)
    (:`0`
      _)
    (:`1`
      _)
    (:`2`
      (`self.K2_SetActorRotation` (`KismetMathLibrary.ComposeRotators` (`self.K2_GetActorRotation`) (`KismetMathLibrary.MakeRotator` 0.0 (`KismetMathLibrary.RandomFloatInRange` -30.0 30.0) (`KismetMathLibrary.RandomFloatInRange` -30.0 30.0))))))
  (`ProjectileMovementComponent.SetVelocityInLocalSpace` (`self.ProjectileMovement`) (1500.0 0.0 0.0))
  (`GameplayStatics.PlaySoundAtLocation` "/Game/Magventures/Sound/Effect/ThrowAxe2.ThrowAxe2" (`self.K2_GetActorLocation`) (struct) 1.0 1.0 0.0 null null null null))

(event `self.ReceiveActorBeginOverlap`
  (params (OtherActor :type "Actor Object Reference"))
  (if (!= OtherActor (`self.GetInstigator`))
    (if (== (`self.ShotResult_0`) 0)
      (`GameplayStatics.PlaySoundAtLocation` "/Engine/EditorSounds/GamePreview/EndPlayInEditor.EndPlayInEditor" (`self.K2_GetActorLocation`) (struct) 1.0 1.0 0.0 null null null null)
      (elif (== (`self.ShotResult_0`) 1)
        (`GameplayStatics.PlaySoundAtLocation` "/Engine/EditorSounds/GamePreview/PossessPlayer.PossessPlayer" (`self.K2_GetActorLocation`) (struct) 1.0 1.0 0.0 null null null null)))
    (`self.K2_DestroyActor`)))

(fn `UserConstructionScript`)